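; BP_Test is a test actor that moves back and forth along its local Y axis after jumping to a fixed transform on BeginPlay.
; Tick accumulates time and, every three seconds, a FlipFlop switches Speed between a negative and a smaller positive value.
; Each other frame offsets Y by Speed times delta time, plus the right vector's Y component, which is added unscaled and so makes movement frame-rate dependent.
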(event `self.ReceiveBeginPlay`
  (`self.K2_SetActorTransform` (`KismetMathLibrary.MakeTransform` (-340.0 440.0 80.0))))

(event `self.ReceiveTick`
  (params (DeltaSeconds :type "Float (single-precision)"))
  (bind _sumtime (`self.SumTime`))
  (bind (_returnvalue_x _returnvalue_y) (`KismetMathLibrary.BreakVector` (+ (* DeltaSeconds (`self.Speed`)) (`self.GetActorRightVector`))))
  (if (>= _sumtime 3.0)
    (`/Engine/EditorBlueprintResources/StandardMacros.FlipFlop`
      (:`A`
        (set `self.Speed` -200.0))
      (:`B`
        (set `self.Speed` 100.0)))
    (set `self.SumTime` 0.0)
    (else
      (set `self.SumTime` (+ DeltaSeconds _sumtime))
      (`self.K2_AddActorLocalOffset` (`KismetMathLibrary.MakeVector` 0.0 _returnvalue_y)))))

(fn `UserConstructionScript`)