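; BP_Monster is a movable monster that wanders at random and chases the player character when it comes within range.
; Tick checks player distance each frame, steering straight at a nearby player by setting rotation and adding movement input.
; Otherwise it follows ToTarget until an accumulated timer expires, pauses through a Delay, then aims at a random point in a square around the world origin.
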(event `self.ReceiveTick`
  (params (DeltaSeconds :type "Float (single-precision)"))
  (bind _returnvalue (- (`self.K2_GetActorLocation` (`GameplayStatics.GetPlayerCharacter` 0)) (`self.K2_GetActorLocation`)))
  (set `self.SumTime` (+ DeltaSeconds (`self.SumTime`)))
  (if (>= (`KismetMathLibrary.VSize` _returnvalue) 1000.0)
    (if (> (`self.SumTime`) 5.0)
      (`KismetSystemLibrary.Delay` 2.0)
      (set `self.ToTarget` (- (`KismetMathLibrary.MakeVector` (`KismetMathLibrary.RandomFloatInRange` -2000.0 2000.0) (`KismetMathLibrary.RandomFloatInRange` -2000.0 2000.0)) (`self.K2_GetActorLocation`)))
      (set `self.SumTime` 0.0)
      (elif (not (`self.bMove`))
        (set `self.bMove` true)
        (`self.K2_SetActorRotation` (`KismetMathLibrary.Conv_VectorToRotator` (`self.ToTarget`)))
        (`self.AddMovementInput` (`self.ToTarget`))
        (set `self.bMove` false)))
    (else
      (set `self.ToTarget` _returnvalue)
      (`self.K2_SetActorRotation` (`KismetMathLibrary.Conv_VectorToRotator` (`self.ToTarget`)))
      (`self.AddMovementInput` (`self.ToTarget`)))))

(fn `UserConstructionScript`)